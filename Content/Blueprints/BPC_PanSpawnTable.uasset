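; Spawn table actor that supplies BPC_Pan items and restocks itself over time.
; On BeginPlay it spawns a pan at its ItemPlacement transform and stores it in SpawnedItem.
; Tick feeds a random-length Delay that acts as a repeating timer, then checks SpawnedItem to decide whether to spawn and store a replacement pan at the same spot.
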(event EventBeginPlay
  (|CallParentFunction)
  ;[0.4417 0.5036 1] Spawning the Pan at the Start
  (bind _returnvalue (Game|SpawnActorfromClass "/Game/Blueprints/BPC_Pan.BPC_Pan_C" (Transformation|GetWorldTransform (Variables|Default|GetItemPlacement)) "AlwaysSpawn" 0 0))
  (Variables|Default|SetSpawned_Item _returnvalue))

(event Collision|EventActorBeginOverlap
  (params (OtherActor :type Actor%20Object%20Reference))
  (|CallParentFunction OtherActor) ; This node is disabled and will not be called.\nDrag off pins to build functionality.
)

(event EventTick
  (params (DeltaSeconds :type Float%20%28single-precision%29))
  (|CallParentFunction DeltaSeconds)
  ;[0.4598 1 0.5456] Setting a Random Timer for the Plate Spawning
  (Utilities|FlowControl|Delay (Math|Random|RandomFloatinRange 8.0 18.0))
  ;[0.3604 1 0.9302] Checking if the Spawn Table already has a Plate
  (if (== (Variables|Default|GetSpawned_Item) 0)
    ;[0.4417 0.5036 1] Spawning the Pan
    (bind _returnvalue (Game|SpawnActorfromClass "/Game/Blueprints/BPC_Pan.BPC_Pan_C" (Transformation|GetWorldTransform (Variables|Default|GetItemPlacement)) "AlwaysSpawn" 0 0))
    (Variables|Default|SetSpawned_Item _returnvalue)))

(fn ConstructionScript
  (|CallParentFunction))