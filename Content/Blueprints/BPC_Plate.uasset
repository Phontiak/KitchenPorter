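; BPC_Plate is a plate actor that other carried items can be stacked on.
; Its Stack event accepts another plate or a pan, detaches it from its current parent and clears the player's Carrying reference.
; The item is then attached to this plate, snapping to its location while keeping world rotation and scale.
; Items of any other type are ignored.
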(event EventBeginPlay
  (|CallParentFunction) ; This node is disabled and will not be called.\nDrag off pins to build functionality.
)

(event Collision|EventActorBeginOverlap
  (params (OtherActor :type Actor%20Object%20Reference))
  (|CallParentFunction OtherActor) ; This node is disabled and will not be called.\nDrag off pins to build functionality.
)

(event EventTick
  (params (DeltaSeconds :type Float%20%28single-precision%29))
  (|CallParentFunction DeltaSeconds) ; This node is disabled and will not be called.\nDrag off pins to build functionality.
)

(event EventStack
  (params (Second_Item :type Actor%20Object%20Reference) (Player_Reference :type BP%20Player%20Character%20Object%20Reference))
  ;[1 1 1] Stacking Plates
  (bind _asbpc_plate (Utilities|Casting|CastToBPC_Plate Second_Item)
    (:then
      (Transformation|DetachFromActor _asbpc_plate "KeepWorld" "KeepWorld" "KeepWorld")
      (Variables|/Game/Blueprints/BP_PlayerCharacter.BP_PlayerCharacter_C|SetCarrying Player_Reference 0)
      (Transformation|AttachActorToActor _asbpc_plate self "None" "SnapToTarget" "KeepWorld" "KeepWorld" true))
    (:CastFailed
      ;[1 1 1] Putting Pans on top of Plates
      (bind _asbpc_pan (Utilities|Casting|CastToBPC_Pan Second_Item))
      (Transformation|DetachFromActor _asbpc_pan "KeepWorld" "KeepWorld" "KeepWorld")
      (Variables|/Game/Blueprints/BP_PlayerCharacter.BP_PlayerCharacter_C|SetCarrying Player_Reference 0)
      (Transformation|AttachActorToActor _asbpc_pan self "None" "SnapToTarget" "KeepWorld" "KeepWorld" true))))

(fn ConstructionScript
  (|CallParentFunction))