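; BP_Item is a washable plate item that moves between Dirty, Washing and Clean states, showing the matching component for each.
; Wash plays a spray sound and starts washing a dirty item, revealing its progress widget.
; Tick advances progress while either of two players is nearby, otherwise reverting to Dirty without resetting progress.
; At full progress it turns Clean, hides the widget and notifies its owning BPC_Sink.
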(event Custom|Wash
  ;[0.2555 0.7775 1 1 30] Show the Washing Progress
  (Audio|PlaySound2D "/Game/Audio/SFX/Water-Sprayer-My-Edit.Water-Sprayer-My-Edit" 1.0 1.0 0.0 0 0)
  (switch Utilities|FlowControl|Switch|SwitchonPlateStates (Variables|Default|GetPlateState)
    (:NewEnumerator2
      (Variables|Default|SetPlateState "NewEnumerator1")
      (Rendering|SetVisibility (Variables|Default|GetWashing_Progress_Widget) true false))))

(event EventBeginPlay
  (bind _aswashing_progress (Utilities|Casting|CastToWashing_Progress (UserInterface|GetUserWidgetObject (Variables|Default|GetWashing_Progress_Widget))))
  (Variables|Default|SetWashing%20Progress _aswashing_progress))

(event EventTick
  (params (DeltaSeconds :type Float%20%28single-precision%29))
  ;[0.3067 0.6052 0.6198 1 30] Controlling the Visibility of the Item States
  (switch Utilities|FlowControl|Switch|SwitchonPlateStates (Variables|Default|GetPlateState)
    (:NewEnumerator0
      (Rendering|SetVisibility (Variables|Default|GetDirty) false true)
      (Rendering|SetVisibility (Variables|Default|GetClean) true true)
      (Rendering|SetVisibility (Variables|Default|GetWashing) false true))
    (:NewEnumerator1
      (Rendering|SetVisibility (Variables|Default|GetDirty) false true)
      (Rendering|SetVisibility (Variables|Default|GetWashing) true true)
      (if (>= (Variables|Default|GetCleaningProgress) 1.0)
        (Variables|Default|SetPlateState "NewEnumerator0")
        (Rendering|SetVisibility (Variables|Default|GetWashing_Progress_Widget) false false)
        (bind _asbpc_sink (Utilities|Casting|CastToBPC_Sink (Variables|Default|GetOwningTable)))
        (Default|ItemFinishedWashing _asbpc_sink self)
        (elif (or (<= (Math|Vector|Distance(Vector) (Transformation|GetActorLocation (Game|GetPlayerCharacter 0)) (Transformation|GetActorLocation)) (Variables|Default|GetWashDistToPlayer)) (<= (Math|Vector|Distance(Vector) (Transformation|GetActorLocation (Game|GetPlayerCharacter 1)) (Transformation|GetActorLocation)) (Variables|Default|GetWashDistToPlayer)))
          ;;[0.5688 1 0.1973 1 23] Updating the Washing Widget
          (bind _output_get (Variables|Default|SetCleaningProgress (+ (Variables|Default|GetCleaningProgress) (* DeltaSeconds (Variables|Default|GetCleanSpeed)))))
          (Variables|/Game/UI/In_Level/Washing_Progress.Washing_Progress_C|SetProgress (Variables|Default|GetWashing%20Progress) _output_get)
          (else
            (Variables|Default|SetPlateState "NewEnumerator2")))))
    (:NewEnumerator2
      (Rendering|SetVisibility (Variables|Default|GetDirty) true true)
      (Rendering|SetVisibility (Variables|Default|GetClean) false true)
      (Rendering|SetVisibility (Variables|Default|GetWashing) false true))))

(fn ConstructionScript)