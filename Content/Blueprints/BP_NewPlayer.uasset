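; Player character for a plate-washing game that moves on world axes, carries items between tables and sinks, and washes plates.
; Overlaps track the current table or sink, which the Pick Up/Drop input uses to attach items to placement or carry points.
; The Washing input calls Wash on the sink's item, and picking up a plate mid-wash resets it to Dirty.
; Tick smoothly rotates the Cube mesh toward the input direction.
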(event EventTick
  (params (DeltaSeconds :type Float%20%28single-precision%29))
  (Utilities|FlowControl|Sequence
    (:then_0
      (CallFunction|RotateChar DeltaSeconds))
    (:then_1
      (Utilities|IsValid (Variables|Default|GetSinkRef)
        (:Is%20Valid
          (bind _asbpnew_item (Utilities|Casting|CastToBPNewItem (Variables|/Game/Blueprints/BP_BasicTable.BP_BasicTable_C|GetItem (Variables|Default|GetSinkRef))))
          (switch Utilities|FlowControl|Switch|SwitchonPlateStates (Variables|/Game/Blueprints/BPNewItem.BPNewItem_C|GetPlateState _asbpnew_item)
            (:NewEnumerator1
              _)
            (:NewEnumerator2
              _))
          (Utilities|FlowControl|Gate true))))))

(event Collision|EventActorBeginOverlap
  (params (OtherActor :type Actor%20Object%20Reference))
  ;[1 1 1] Player Overlapping with the tables
  (bind _asbpc_sink (Utilities|Casting|CastToBPC_Sink OtherActor)
    (:then
      (Variables|Default|SetSinkRef _asbpc_sink))
    (:CastFailed
      (bind _asbp_basic_table (Utilities|Casting|CastToBP_BasicTable OtherActor))
      (Variables|Default|SetTableRef _asbp_basic_table))))

(event Collision|EventActorEndOverlap
  (params (OtherActor :type Actor%20Object%20Reference))
  ;[1 1 1] Player Overlapping with the tables
  (Utilities|Casting|CastToBPC_Sink OtherActor
    (:then
      (Variables|Default|SetSinkRef 0))
    (:CastFailed
      (bind _asbp_basic_table (Utilities|Casting|CastToBP_BasicTable OtherActor))
      (if (Utilities|Enum|Equal(Enum) (Utilities|GetObjectName (Variables|Default|GetTableRef)) (Utilities|GetObjectName _asbp_basic_table))
        (Variables|Default|SetTableRef 0)))))

(event EventBeginPlay
  (bind _charactermovement (Variables|Character|GetCharacterMovement))
  (Variables|/Script/Engine.CharacterMovementComponent|SetMaxStepHeight _charactermovement 1e+01)
  (Variables|/Script/Engine.CharacterMovementComponent|SetMaxWalkSpeed _charactermovement 5e+02))

(event Input|ActionEvents|InputActionPickUp/Drop
  (params (Key :type Key%20Structure :default "None"))
  (bind _tableref (Variables|Default|GetTableRef))
  (bind _tableref_2 (Variables|Default|GetTableRef))
  (bind _sinkref (Variables|Default|GetSinkRef))
  (bind _sinkref_2 (Variables|Default|GetSinkRef))
  (:Pressed
    (Utilities|IsValid (Variables|Default|GetCarrying)
      (:Is%20Valid
        ;[1 1 1] Drop Items
        (Utilities|IsValid _sinkref
          (:Is%20Valid
            (Utilities|IsValid (Variables|/Game/Blueprints/BP_BasicTable.BP_BasicTable_C|GetItem _sinkref)
              (:Is%20Not%20Valid
                (Transformation|DetachFromActor (Variables|Default|GetCarrying) "KeepWorld" "KeepWorld" "KeepWorld")
                (bind _output_get (Variables|/Game/Blueprints/BP_BasicTable.BP_BasicTable_C|SetItem _sinkref_2 (Variables|Default|GetCarrying)))
                (bind _asbpnew_item (Utilities|Casting|CastToBPNewItem (Variables|Default|GetCarrying)))
                (Variables|/Game/Blueprints/BPNewItem.BPNewItem_C|SetOwningTable _asbpnew_item (Variables|Default|GetSinkRef))
                (Transformation|AttachComponentToComponent _output_get (Variables|/Game/Blueprints/BP_BasicTable.BP_BasicTable_C|GetItemPlacement _sinkref_2) "None" "SnapToTarget" "KeepWorld" "KeepWorld" true)
                (Variables|Default|SetCarrying 0))))
          (:Is%20Not%20Valid
            (Utilities|IsValid _tableref
              (:Is%20Valid
                (Utilities|IsValid (Variables|/Game/Blueprints/BP_BasicTable.BP_BasicTable_C|GetItem _tableref)
                  (:Is%20Not%20Valid
                    (Transformation|DetachFromActor (Variables|Default|GetCarrying) "KeepWorld" "KeepWorld" "KeepWorld")
                    (bind _output_get_2 (Variables|/Game/Blueprints/BP_BasicTable.BP_BasicTable_C|SetItem _tableref_2 (Variables|Default|GetCarrying)))
                    (Transformation|AttachComponentToComponent _output_get_2 (Variables|/Game/Blueprints/BP_BasicTable.BP_BasicTable_C|GetItemPlacement _tableref_2) "None" "SnapToTarget" "KeepWorld" "KeepWorld" true)
                    (Variables|Default|SetCarrying 0))))))))
      (:Is%20Not%20Valid
        ;[1 1 1] Pick Up Items
        (Utilities|IsValid (Variables|Default|GetTableRef)
          (:Is%20Valid
            (Utilities|IsValid (Variables|/Game/Blueprints/BP_BasicTable.BP_BasicTable_C|GetItem (Variables|Default|GetTableRef))
              (:Is%20Valid
                (Variables|Default|SetCarrying (Variables|/Game/Blueprints/BP_BasicTable.BP_BasicTable_C|GetItem (Variables|Default|GetTableRef)))
                (Transformation|DetachFromActor (Variables|/Game/Blueprints/BP_BasicTable.BP_BasicTable_C|GetItem (Variables|Default|GetTableRef)) "KeepWorld" "KeepWorld" "KeepWorld")
                (Variables|/Game/Blueprints/BP_BasicTable.BP_BasicTable_C|SetItem (Variables|Default|GetTableRef) 0)
                (Transformation|AttachComponentToComponent (Variables|Default|GetCarrying) (Variables|Default|GetCarryingPosition) "None" "SnapToTarget" "KeepWorld" "KeepWorld" true))))
          (:Is%20Not%20Valid
            (Utilities|IsValid (Variables|Default|GetSinkRef)
              (:Is%20Valid
                (Utilities|IsValid (Variables|/Game/Blueprints/BP_BasicTable.BP_BasicTable_C|GetItem (Variables|Default|GetSinkRef))
                  (:Is%20Valid
                    (Variables|Default|SetCarrying (Variables|/Game/Blueprints/BP_BasicTable.BP_BasicTable_C|GetItem (Variables|Default|GetSinkRef)))
                    (Transformation|DetachFromActor (Variables|/Game/Blueprints/BP_BasicTable.BP_BasicTable_C|GetItem (Variables|Default|GetSinkRef)) "KeepWorld" "KeepWorld" "KeepWorld")
                    (Variables|/Game/Blueprints/BP_BasicTable.BP_BasicTable_C|SetItem (Variables|Default|GetSinkRef) 0)
                    (Transformation|AttachComponentToComponent (Variables|Default|GetCarrying) (Variables|Default|GetCarryingPosition) "None" "SnapToTarget" "KeepWorld" "KeepWorld" true)))))))
        (bind _asbpnew_item_2 (Utilities|Casting|CastToBPNewItem (Variables|Default|GetCarrying)))
        (switch Utilities|FlowControl|Switch|SwitchonPlateStates (Variables|/Game/Blueprints/BPNewItem.BPNewItem_C|GetPlateState _asbpnew_item_2)
          (:NewEnumerator1
            _)
          (:NewEnumerator2
            _))
        (Variables|/Game/Blueprints/BPNewItem.BPNewItem_C|SetPlateState _asbpnew_item_2 "NewEnumerator2")))))

(event Input|ActionEvents|InputActionWashing
  (params (Key :type Key%20Structure :default "None"))
  (:Pressed
    (bind _asbpnew_item (Utilities|Casting|CastToBPNewItem (Variables|/Game/Blueprints/BP_BasicTable.BP_BasicTable_C|GetItem (Variables|Default|GetSinkRef))))
    (Default|Wash _asbpnew_item)))

(event Input|ActionEvents|InputActionWashing
  (params (Key :type Key%20Structure :default "None"))
  (:Pressed
    (Utilities|FlowControl|Gate true) ; enters at Open
  ))

(event Input|AxisEvents|InputAxisUpDown
  (params (AxisValue :type Float%20%28single-precision%29))
  ;[1 1 1] Player movement inputs
  (Pawn|Input|AddMovementInput "1.000000, 0, 0" AxisValue false))

(event Input|AxisEvents|InputAxisLeftRight
  (params (AxisValue :type Float%20%28single-precision%29))
  ;[1 1 1] Player movement inputs
  (Pawn|Input|AddMovementInput "0,1.000000, 0" AxisValue false))

(fn ConstructionScript)

(fn RotateChar
  (params (InputPin :type Float%20%28single-precision%29))
  (if (or (!= (Input|AxisValues|GetUpDown) 0.0) (!= (Input|AxisValues|GetLeftRight) 0.0))
    ;[1 1 1] Set wanted direction
    (Variables|Default|SetDirection (Math|Vector|MakeVector (Input|AxisValues|GetUpDown) (Input|AxisValues|GetLeftRight) 0.0))
    (Transformation|SetWorldRotation (Variables|Default|GetCube) (Math|Rotator|Lerp(Rotator) (Transformation|GetWorldRotation (Variables|Default|GetCube)) (Math|Conversions|RotationFromXVector (Variables|Default|GetDirection)) (* InputPin (Variables|Default|GetRotationSpeed)) true) false false)))