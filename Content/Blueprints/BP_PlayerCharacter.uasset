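; Player character that moves on world axes and carries items between tables, picking up, placing or stacking them.
; Tick smoothly turns the Cube toward the input direction and sphere-traces ahead of it, with debug drawing, to find what is in reach.
; The Pick Up/Drop action passes that hit to TableFunctions, which re-attaches items between CarryingPosition and the table's ItemPlacement, or calls Stack when both hold one.
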(event EventTick
  (params (DeltaSeconds :type Float%20%28single-precision%29))
  (bind _cube (Variables|Default|GetCube))
  (bind _returnvalue (Transformation|GetWorldLocation _cube))
  (if (or (!= (Input|AxisValues|GetUpDown) 0.0) (!= (Input|AxisValues|GetLeftRight) 0.0))
    ;[1 1 1] Set wanted direction
    (Variables|Default|SetDirection (Math|Vector|MakeVector (Input|AxisValues|GetUpDown) (Input|AxisValues|GetLeftRight) 0.0))
    (Transformation|SetWorldRotation (Variables|Default|GetCube) (Math|Rotator|Lerp(Rotator) (Transformation|GetWorldRotation (Variables|Default|GetCube)) (Math|Conversions|RotationFromXVector (Variables|Default|GetDirection)) (* DeltaSeconds (Variables|Default|GetRotationSpeed)) true) false false))
  (bind _outhit (Collision|SphereTraceByChannel _returnvalue (+ _returnvalue (* (Math|Vector|GetForwardVector _cube) (Variables|Default|GetGrabRange))) (Variables|Default|GetGrabRadius) "TraceTypeQuery1" false 0 "ForOneFrame")))

(event Input|ActionEvents|InputActionPickUp/Drop
  (params (Key :type Key%20Structure))
  (:Pressed
    (CallFunction|TableFunctions (.HitActor (Collision|BreakHitResult (stale EventTick _outhit))))))

(event Input|AxisEvents|InputAxisUpDown
  (params (AxisValue :type Float%20%28single-precision%29))
  ;[1 1 1] Player movement inputs
  (Pawn|Input|AddMovementInput "1.000000, 0, 0" AxisValue false))

(event Input|AxisEvents|InputAxisLeftRight
  (params (AxisValue :type Float%20%28single-precision%29))
  ;[1 1 1] Player movement inputs
  (Pawn|Input|AddMovementInput "0,1.000000, 0" AxisValue false))

(fn ConstructionScript)

(fn TableFunctions
  (params (Table :type Actor%20Object%20Reference))
  (bind _asbp_basic_table (Utilities|Casting|CastToBP_BasicTable Table))
  (Utilities|IsValid (Variables|/Game/Blueprints/BP_BasicTable.BP_BasicTable_C|GetItem _asbp_basic_table)
    (:Is%20Valid
      (Utilities|IsValid (Variables|Default|GetCarrying)
        (:Is%20Valid
          ;[1 1 1] Stack Items
          (bind _asbp_item (Utilities|Casting|CastToBP_Item (Variables|/Game/Blueprints/BP_BasicTable.BP_BasicTable_C|GetItem _asbp_basic_table)))
          (Default|Stack _asbp_item (Variables|Default|GetCarrying) self))
        (:Is%20Not%20Valid
          ;[1 1 1] Pick up from the table
          (Transformation|DetachFromActor (Variables|/Game/Blueprints/BP_BasicTable.BP_BasicTable_C|GetItem _asbp_basic_table) "KeepWorld" "KeepWorld" "KeepWorld")
          (bind _output_get (Variables|Default|SetCarrying (Variables|/Game/Blueprints/BP_BasicTable.BP_BasicTable_C|GetItem _asbp_basic_table)))
          (Transformation|AttachComponentToComponent _output_get (Variables|Default|GetCarryingPosition) "None" "SnapToTarget" "KeepWorld" "KeepWorld" true)
          (Variables|/Game/Blueprints/BP_BasicTable.BP_BasicTable_C|SetItem _asbp_basic_table 0))))
    (:Is%20Not%20Valid
      (Utilities|IsValid (Variables|Default|GetCarrying)
        (:Is%20Valid
          ;[1 1 1] Place down on a table
          (Transformation|DetachFromActor (Variables|Default|GetCarrying) "KeepWorld" "KeepWorld" "KeepWorld")
          (Transformation|AttachComponentToComponent (Variables|Default|GetCarrying) (Variables|/Game/Blueprints/BP_BasicTable.BP_BasicTable_C|GetItemPlacement _asbp_basic_table) "None" "SnapToTarget" "KeepWorld" "KeepWorld" true)
          (Variables|/Game/Blueprints/BP_BasicTable.BP_BasicTable_C|SetItem _asbp_basic_table (Variables|Default|GetCarrying))
          (Variables|Default|SetCarrying 0))))))