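; Game mode for the single-player main level that spawns players, runs a countdown timer and tracks score.
; BeginPlay adds Timer and Score widgets, then spawns and possesses a BP_PlayerCharacter at each PlayerStart whose tag matches a player index.
; Tick uses a one-second Delay to step the minutes and seconds countdown, showing Level_Finish and pausing at zero.
; ScoreCount adds the given amount to Points.
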(event EventBeginPlay
  (Utilities|FlowControl|Sequence
    (:then_0
      (bind _returnvalue (UserInterface|CreateWidget "/Game/UI/Timer.Timer_C"))
      (UserInterface|Viewport|AddtoViewport _returnvalue 0)
      ;[0.3836 1 0.2325 1 20] Spawning Players
      (CallFunction|PlayersSpawnLocations)
      (CallFunction|SpawnPlayers))
    (:then_1
      (bind _returnvalue_2 (UserInterface|CreateWidget "/Game/UI/Score.Score_C"))
      (UserInterface|Viewport|AddtoViewport _returnvalue_2 0)
      ;[1 0.7981 0.2486 1 20] Score System
      (CallFunction|ScoreCount))))

(event EventTick
  (params (DeltaSeconds :type Float%20%28single-precision%29))
  ;[0.3412 0.3927 1 1 20] Timer
  (Utilities|FlowControl|Delay 1.0)
  (CallFunction|CountdownTimer))

(fn ConstructionScript)

(fn PlayersSpawnLocations
  (bind _outactors (Actor|GetAllActorsOfClass "/Script/Engine.PlayerStart"))
  (Variables|Default|SetPlayerSpawnLocationArray _outactors))

(fn SpawnPlayers
  (for _index (range 0 (- (Variables|Default|GetMaxNumberOfPlayers) 1))
    (Variables|Default|SetIndex _index)
    (for _array_element (Variables|Default|GetPlayerSpawnLocationArray)
      (if (Utilities|Name|Equal(Name) (Variables|/Script/Engine.PlayerStart|GetPlayerStartTag _array_element) (Utilities|String|StringToName (Utilities|String|ToString(Integer) (Variables|Default|GetIndex))))
        (Class|GameplayStatics|CreatePlayer (Variables|Default|GetIndex))
        (bind _returnvalue (Game|SpawnActorfromClass "/Game/Blueprints/BP_PlayerCharacter.BP_PlayerCharacter_C" (Transformation|GetActorTransform _array_element) "AlwaysSpawn" 0 0))
        (Pawn|Possess (Game|GetPlayerController (Variables|Default|GetIndex)) _returnvalue)))))

(fn CountdownTimer
  (if (== (Variables|Default|GetSeconds) 0)
    (if (== (Variables|Default|GetMinutes) 0)
      ;[1 1 1] Ran out of time
      (bind _returnvalue (UserInterface|CreateWidget "/Game/UI/Level_Finish.Level_Finish_C"))
      (UserInterface|Viewport|AddtoViewport _returnvalue 0)
      (Variables|/Script/Engine.PlayerController|SetbShowMouseCursor (Game|GetPlayerController 0) true)
      (Game|SetGamePaused true)
      (else
        (Variables|Default|SetSeconds 59)
        (bind _result (Math|Integer|DecrementInt (Variables|Default|GetMinutes))
          (:%20%20
            (Variables|Default|SetMinutes _result)))))
    (else
      (bind _result_2 (Math|Integer|DecrementInt (Variables|Default|GetSeconds))
        (:%20%20
          (Variables|Default|SetSeconds _result_2))))))

(fn ScoreCount
  (params (Score%20ammount :type Integer))
  (Variables|Default|SetPoints (+ (Variables|Default|GetPoints) Score%20ammount)))