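; Game mode for the level select menu that spawns the local players when play begins.
; It first gathers every PlayerStart in the level.
; For each index below MaxNumberOfPlayers, it finds starts tagged with that number, creates a local player, spawns a BP_PlayerCharacter there regardless of collision and has that player's controller possess it.
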(event EventBeginPlay
  ;[0.3836 1 0.2325 1 20] Spawning Players
  (CallFunction|PlayersSpawnLocations)
  (CallFunction|SpawnPlayers))

(event EventTick
  (params (DeltaSeconds :type Float%20%28single-precision%29)))

(fn ConstructionScript)

(fn PlayersSpawnLocations
  (bind _outactors (Actor|GetAllActorsOfClass "/Script/Engine.PlayerStart"))
  (Variables|Default|SetPlayerSpawnLocationArray _outactors))

(fn SpawnPlayers
  (for _index (range 0 (- (Variables|Default|GetMaxNumberOfPlayers) 1))
    (Variables|Default|SetIndex _index)
    (for _array_element (Variables|Default|GetPlayerSpawnLocationArray)
      (if (Utilities|Name|Equal(Name) (Variables|/Script/Engine.PlayerStart|GetPlayerStartTag _array_element) (Utilities|String|StringToName (Utilities|String|ToString(Integer) (Variables|Default|GetIndex))))
        (Class|GameplayStatics|CreatePlayer (Variables|Default|GetIndex))
        (bind _returnvalue (Game|SpawnActorfromClass "/Game/Blueprints/BP_PlayerCharacter.BP_PlayerCharacter_C" (Transformation|GetActorTransform _array_element) "AlwaysSpawn" 0 0))
        (Pawn|Possess (Game|GetPlayerController (Variables|Default|GetIndex)) _returnvalue)))))